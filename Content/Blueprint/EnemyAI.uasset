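; Enemy AI that picks a random Cows actor at BeginPlay, walks toward it and attacks cows it touches.
; AIMoveTo tracks the moving target continuously, while Tick turns the enemy's yaw to face it.
; Overlap events record the touched actor, and Tick applies damage to it whenever the accumulated cooldown exceeds the attack rate, provided its class is exactly Cows.
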(event `self.ReceiveBeginPlay`
  (bind _outactors (`GameplayStatics.GetAllActorsOfClass` "/Game/Blueprint/Cows.Cows_C"))
  (bind _output_get (set `self.way points` _outactors))
  (set `self.target` (`|GetArrayItem` _output_get (`KismetMathLibrary.RandomIntegerInRange` 0 (- (`KismetArrayLibrary.Array_Length` _output_get) 1))))
  (`AITask_MoveTo.AIMoveTo` (`AIBlueprintHelperLibrary.GetAIController` self) (0.0 0.0 0.0) (`self.target`) -1.0 "Disable" "Default" true true true
    (:`then`
      (set `self.attackRate` 2.0)
      (set `self.damage` 10.0))))

(event `self.ReceiveTick`
  (params (DeltaSeconds :type "Float (single-precision)"))
  (bind (_returnvalue_roll _returnvalue_pitch _returnvalue_yaw) (`KismetMathLibrary.BreakRotator` (`KismetMathLibrary.FindLookAtRotation` (`SceneComponent.K2_GetComponentLocation` (`self.RootComponent`)) (`self.K2_GetActorLocation` (`self.target`)))))
  (`self.K2_SetActorRotation` self (`KismetMathLibrary.MakeRotator` 0.0 0.0 _returnvalue_yaw) false)
  (set `self.attackCooldown` (+ (* 1.0 DeltaSeconds) (`self.attackCooldown`)))
  (if (`self.isOverlapping`)
    (if (== "/Game/Blueprint/Cows.Cows_C" (`GameplayStatics.GetObjectClass` (`self.overlapActor`)))
      (if (> (`self.attackCooldown`) (`self.attackRate`))
        (`GameplayStatics.ApplyDamage` (`self.overlapActor`) (`self.damage`))
        (set `self.attackCooldown` 0.0)))))

(event `self.ReceiveActorBeginOverlap`
  (params (OtherActor :type "Actor Object Reference"))
  (set `self.isOverlapping` true)
  (set `self.overlapActor` OtherActor))

(event `self.ReceiveActorEndOverlap`
  (params (OtherActor :type "Actor Object Reference"))
  (set `self.isOverlapping` false))

(event `self.ReceiveAnyDamage`
  (params (Damage :type "Float (single-precision)") (DamageType :type "DamageType Object Reference") (InstigatedBy :type "Controller Object Reference") (DamageCauser :type "Actor Object Reference")))

(fn `UserConstructionScript`)