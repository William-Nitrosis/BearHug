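; BulletProjectile is a projectile actor that appears as a random novelty object and damages enemies.
; On BeginPlay it picks one of several meshes, such as a cupcake, cactus or banana, and rescales RandomBody by matching the mesh's display name.
; On overlap it applies fixed damage to EnemyAI actors.
; It destroys itself on overlapping anything except the PlayerCharacter or another BulletProjectile, using exact class comparisons.
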(event `self.ReceiveBeginPlay`
  (bind _randombody (`self.randomBody`))
  (set `self.damage` 20.0)
  (bind _output_get (set `self.bulletMeshes` (`|MakeArray` "/Game/Meshes/SM_Cupcake.SM_Cupcake" "/Game/Meshes/SM_Cactus.SM_Cactus" "/Game/Meshes/SM_Gun.SM_Gun" "/Game/Meshes/SM_Horseshoe_01a.SM_Horseshoe_01a" "/Game/Meshes/SM_Satellite_01a.SM_Satellite_01a" "/Game/Meshes/SM_Single_Planet_01a.SM_Single_Planet_01a" "/Game/Meshes/SM_Tree.SM_Tree" "/Game/Meshes/SM_Une_Banane_01a.SM_Une_Banane_01a" :!type "StaticMesh Object Reference")))
  (set `self.theMesh` (`|GetArrayItem` _output_get (`KismetMathLibrary.RandomIntegerInRange` 0 (- (`KismetArrayLibrary.Array_Length` _output_get) 1))))
  (switch `string` (`KismetSystemLibrary.GetDisplayName` (`self.theMesh`))
    (:`sm_cupcake`
      (`SceneComponent.SetWorldScale3D` _randombody (1.0 1.0 1.0)))
    (:`sm_cactus`
      (`SceneComponent.SetWorldScale3D` _randombody (0.5 0.5 0.5)))
    (:`sm_gun`
      (`SceneComponent.SetWorldScale3D` _randombody (0.15625 0.15625 0.15625)))
    (:`sm_horseshoe_01a`
      (`SceneComponent.SetWorldScale3D` _randombody (0.65 0.65 0.65)))
    (:`sm_single_planet_01a`
      (`SceneComponent.SetWorldScale3D` _randombody (0.4 0.4 0.4)))
    (:`sm_satelite_01a`
      (`SceneComponent.SetWorldScale3D` _randombody (0.25 0.25 0.25)))
    (:`sm_tree`
      (`SceneComponent.SetWorldScale3D` _randombody (0.15625 0.15625 0.15625)))
    (:`SM_Une_Banane_01a`
      (`SceneComponent.SetWorldScale3D` _randombody (0.5 0.5 0.5))))
  (`StaticMeshComponent.SetStaticMesh` (`self.randomBody`) (`self.theMesh`)))

(event `self.ReceiveActorBeginOverlap`
  (params (OtherActor :type "Actor Object Reference"))
  (if (== "/Game/Blueprint/EnemyAI.EnemyAI_C" (`GameplayStatics.GetObjectClass` OtherActor))
    (`GameplayStatics.ApplyDamage` OtherActor (`self.damage`)))
  (if (not (or (== "/Game/Blueprint/PlayerCharacter.PlayerCharacter_C" (`GameplayStatics.GetObjectClass` OtherActor)) (== "BulletProjectile_C" (`GameplayStatics.GetObjectClass` OtherActor))))
    (`self.K2_DestroyActor`)))

(fn `UserConstructionScript`)