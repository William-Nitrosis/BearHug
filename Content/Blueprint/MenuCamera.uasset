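; MenuCamera is the main menu actor, turning player input into selections on a UI_Menu widget held by its Widget component.
; The dUp and dDown actions set the widget's Selected index to the first or second option.
; The jump action confirms, opening the Default level for the first option and quitting the game otherwise.
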(event `self.ReceiveBeginPlay`)

(event `InputAction|dUp`
  (params (Key :type "Key Structure"))
  (:`Pressed`
    (bind _asui_menu (cast `/Game/UI/UI_Menu` (`WidgetComponent.GetUserWidgetObject` (`self.Widget`))))
    (set `/Game/UI/UI_Menu.selected` 0 _asui_menu)))

(event `InputAction|dDown`
  (params (Key :type "Key Structure"))
  (:`Pressed`
    (bind _asui_menu (cast `/Game/UI/UI_Menu` (`WidgetComponent.GetUserWidgetObject` (`self.Widget`))))
    (set `/Game/UI/UI_Menu.selected` 1 _asui_menu)))

(event `InputAction|jump`
  (params (Key :type "Key Structure"))
  (:`Pressed`
    (bind _asui_menu (cast `/Game/UI/UI_Menu` (`WidgetComponent.GetUserWidgetObject` (`self.Widget`))))
    (if (== (`/Game/UI/UI_Menu.selected` _asui_menu) 0)
      (`GameplayStatics.OpenLevel` "Default")
      (else
        (`KismetSystemLibrary.QuitGame` null "Quit")))))

(fn `UserConstructionScript`)