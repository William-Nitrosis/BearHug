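; Camera Blueprint that runs the wave loop, alternating timed setup and wave phases stored in DefaultGameInst.
; Tick counts down the timer, flips the phase on expiry and increments the wave as each wave phase begins.
; It pushes timer, banner flags, wave number and live EnemyAI and Cows counts to UI_Overlay.
; A resettable DoOnce triggers aiSpawner once per wave, and EndLevel opens when no cows remain.
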(event `self.ReceiveBeginPlay`
  (bind _output_get (set `self.time` 0.0))
  (bind _output_get_2 (set `self.phase1Time` 5.0))
  (set `self.phase2Time` 60.0)
  (set `self.timeLeft` (- _output_get_2 _output_get))
  (bind _asui_overlay (cast `/Game/UI/UI_Overlay` (`WidgetComponent.GetUserWidgetObject` (`self.UI`))))
  (set `/Game/UI/UI_Overlay.currentWave` 0 _asui_overlay)
  (set `/Game/UI/UI_Overlay.aiAlive` 0 _asui_overlay)
  (set `/Game/UI/UI_Overlay.cowsAlive` 0 _asui_overlay))

(event `self.ReceiveTick`
  (params (DeltaSeconds :type "Float (single-precision)"))
  (bind _timeleft (`self.timeLeft`))
  (bind _timeleft_2 (`self.timeLeft`))
  (bind _returnvalue (`WidgetComponent.GetUserWidgetObject` (`self.UI`)))
  (bind _returnvalue_2 (`WidgetComponent.GetUserWidgetObject` (`self.UI`)))
  (bind _asdefault_game_inst (cast `/Game/Blueprint/DefaultGameInst` (`GameplayStatics.GetGameInstance`)))
  (if (and (== (`/Game/Blueprint/DefaultGameInst.phase` _asdefault_game_inst) 0) (< (`KismetMathLibrary.FFloor` (`self.timeLeft`)) 0))
    (set `/Game/Blueprint/DefaultGameInst.phase` 1 _asdefault_game_inst)
    (set `self.time` 0.0)
    (set `self.timeLeft` 30.0)
    (bind _asui_overlay (cast `/Game/UI/UI_Overlay` (`WidgetComponent.GetUserWidgetObject` (`self.UI`))))
    (bind _result (`/Engine/EditorBlueprintResources/StandardMacros.IncrementInt` (`/Game/UI/UI_Overlay.currentWave` _asui_overlay))
      (:`  `
        (set `/Game/UI/UI_Overlay.currentWave` _result _asui_overlay)))
    (elif (< (`KismetMathLibrary.FFloor` (`self.timeLeft`)) 0)
      (set `/Game/Blueprint/DefaultGameInst.phase` 0 _asdefault_game_inst)
      (set `self.time` 0.0)
      (set `self.timeLeft` 10.0)))
  (set `self.timeLeft` (- _timeleft_2 (* DeltaSeconds 1.0)))
  (if (< (`KismetMathLibrary.FFloor` _timeleft_2) 10)
    (bind _asui_overlay_2 (cast `/Game/UI/UI_Overlay` (`WidgetComponent.GetUserWidgetObject` (`self.UI`))))
    (set `/Game/UI/UI_Overlay.timerVar` (`KismetTextLibrary.Conv_StringToText` (`KismetStringLibrary.Concat_StrStr` "0" (`KismetTextLibrary.Conv_TextToString` (`KismetTextLibrary.Conv_DoubleToText` (`KismetMathLibrary.Conv_IntToDouble` (`KismetMathLibrary.FFloor` _timeleft)) "HalfToEven")))) _asui_overlay_2)
    (else
      (bind _asui_overlay_3 (cast `/Game/UI/UI_Overlay` (`WidgetComponent.GetUserWidgetObject` (`self.UI`))))
      (set `/Game/UI/UI_Overlay.timerVar` (`KismetTextLibrary.Conv_DoubleToText` (`KismetMathLibrary.Conv_IntToDouble` (`KismetMathLibrary.FFloor` _timeleft)) "HalfToEven") _asui_overlay_3)))
  (bind _asdefault_game_inst_2 (cast `/Game/Blueprint/DefaultGameInst` (`GameplayStatics.GetGameInstance`))
    (:`then`
      _)
    (:`CastFailed`
      _))
  (if (and (== (`/Game/Blueprint/DefaultGameInst.phase` _asdefault_game_inst_2) 1) (> (`self.timeLeft`) 57.0))
    (bind _asui_overlay_4 (cast `/Game/UI/UI_Overlay` _returnvalue_2))
    (set `/Game/UI/UI_Overlay.waveDisplay` true _asui_overlay_4)
    (else
      (bind _asui_overlay_5 (cast `/Game/UI/UI_Overlay` _returnvalue_2))
      (set `/Game/UI/UI_Overlay.waveDisplay` false _asui_overlay_5)))
  (bind _asdefault_game_inst_3 (cast `/Game/Blueprint/DefaultGameInst` (`GameplayStatics.GetGameInstance`))
    (:`then`
      _)
    (:`CastFailed`
      _))
  (if (== (`/Game/Blueprint/DefaultGameInst.phase` _asdefault_game_inst_3) 0)
    (bind _asui_overlay_6 (cast `/Game/UI/UI_Overlay` _returnvalue))
    (set `/Game/UI/UI_Overlay.setupDisplay` true _asui_overlay_6)
    (else
      (bind _asui_overlay_7 (cast `/Game/UI/UI_Overlay` _returnvalue))
      (set `/Game/UI/UI_Overlay.setupDisplay` false _asui_overlay_7)))
  (bind _asui_overlay_8 (cast `/Game/UI/UI_Overlay` (`WidgetComponent.GetUserWidgetObject` (`self.UI`))))
  (bind _outactors (`GameplayStatics.GetAllActorsOfClass` "/Game/Blueprint/EnemyAI.EnemyAI_C"))
  (set `/Game/UI/UI_Overlay.aiAlive` (`KismetArrayLibrary.Array_Length` _outactors) _asui_overlay_8)
  (bind _outactors_2 (`GameplayStatics.GetAllActorsOfClass` "/Game/Blueprint/Cows.Cows_C"))
  (bind _asui_overlay_9 (cast `/Game/UI/UI_Overlay` (`WidgetComponent.GetUserWidgetObject` (`self.UI`))))
  (bind _returnvalue_3 (`KismetArrayLibrary.Array_Length` _outactors_2))
  (set `/Game/UI/UI_Overlay.cowsAlive` _returnvalue_3 _asui_overlay_9)
  (if (<= _returnvalue_3 0)
    (`GameplayStatics.OpenLevel` "EndLevel"))
  (bind _asdefault_game_inst_4 (cast `/Game/Blueprint/DefaultGameInst` (`GameplayStatics.GetGameInstance`)))
  (set `/Game/Blueprint/DefaultGameInst.waveCount` (`/Game/UI/UI_Overlay.currentWave` _asui_overlay_9) _asdefault_game_inst_4)
  (bind _asdefault_game_inst_5 (cast `/Game/Blueprint/DefaultGameInst` (`GameplayStatics.GetGameInstance`)))
  (if (== (`/Game/Blueprint/DefaultGameInst.phase` _asdefault_game_inst_5) 1)
    (`/Engine/EditorBlueprintResources/StandardMacros.DoOnce` false :!label _label
      (:`Completed`
        (bind _asai_spawner (cast `/Game/Blueprint/aiSpawner` (`self.aiSpawnerRef`)))
        (`/Game/Blueprint/aiSpawner.spawnAi` _asai_spawner)))
    (else
      (goto _label :!via `Reset`))))

(fn `UserConstructionScript`)