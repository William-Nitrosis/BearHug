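; Cow Character with a health bar widget updated each tick and a randomly chosen green, pink or purple body material at spawn.
; While its Pushed flag is set, it moves directly away from the stored Player reference and turns its mesh that way.
; Damage lowers health, destroying the cow below 1, otherwise launching it in a random upward direction with a half-second material flash.
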(event `setPlayerObjRef`
  (params (player :type "/Game/Blueprint/PlayerCharacter Object Reference"))
  (set `self.player` player))

(event `self.ReceiveTick`
  (params (DeltaSeconds :type "Float (single-precision)"))
  (bind _returnvalue (`KismetMathLibrary.Normal` (- (`self.K2_GetActorLocation` self) (`self.K2_GetActorLocation` (`self.player`)))))
  (`|ExecutionSequence`
    (:`then_0`
      (bind _ashealth_bar (cast `/Game/UI/healthBar` (`WidgetComponent.GetUserWidgetObject` (`self.HealthUI`))))
      (`ProgressBar.SetPercent` (`/Game/UI/healthBar.ProgressBar_88` _ashealth_bar) (/ (`self.health`) 100.0)))
    (:`then_1`
      (if (`self.pushed?`)
        (`self.AddMovementInput` _returnvalue 5.0)
        (`SceneComponent.K2_SetWorldRotation` (`self.Mesh`) (`KismetMathLibrary.Conv_VectorToRotator` _returnvalue) false false)))))

(event `self.ReceiveBeginPlay`
  (switch `int` (`KismetMathLibrary.RandomIntegerInRange` 0 3)
    (:`0`
      (set `self.mat` "/Game/Meshes/CowGreen.CowGreen"))
    (:`1`
      (set `self.mat` "/Game/Meshes/CowPink.CowPink"))
    (:`2`
      (set `self.mat` "/Game/Meshes/CowPurple.CowPurple")))
  (`PrimitiveComponent.SetMaterial` (`self.Body`) 0 (`self.mat`)))

(event `self.ReceiveAnyDamage`
  (params (Damage :type "Float (single-precision)") (DamageType :type "DamageType Object Reference") (InstigatedBy :type "Controller Object Reference") (DamageCauser :type "Actor Object Reference"))
  (set `self.health` (- (`self.health`) Damage))
  (if (< (`self.health`) 1.0)
    (`self.K2_DestroyActor` self)
    (else
      (`PrimitiveComponent.SetMaterial` (`self.Body`) 0 "/Engine/MapTemplates/Materials/BasicAsset01.BasicAsset01")
      (`self.LaunchCharacter` (`KismetMathLibrary.MakeVector` (`KismetMathLibrary.RandomFloatInRange` -350.0 350.0) (`KismetMathLibrary.RandomFloatInRange` -350.0 350.0) 350.0))
      (`KismetSystemLibrary.Delay` 0.5)
      (`PrimitiveComponent.SetMaterial` (`self.Body`) 0 (`self.mat`)))))

(fn `UserConstructionScript`)