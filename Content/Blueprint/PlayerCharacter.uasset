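; Player character Blueprint for cursor-aimed movement with a fixed view target and visible mouse cursor.
; Both input axes share one path that adds control-yaw forward and right movement together, negated when Damage exceeds InvertDamage.
; BeginPlay sets up the camera, cursor and damage values, though nothing here raises Damage afterwards.
; Tick traces under the cursor, yaws the actor using a look-at from the controller's location, and moves a decal to the hit point.
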(event `InputAxis|forwardAxis`
  (params (AxisValue :type "Float (single-precision)"))
  (bind _returnvalue (`KismetMathLibrary.MakeRotator` 0.0 0.0 (.yaw (`self.GetControlRotation`))))
  (bind _returnvalue_2 (`KismetMathLibrary.GetForwardVector` _returnvalue))
  (bind _returnvalue_3 (`KismetMathLibrary.GetRightVector` _returnvalue))
  ;[1 1 1] Movement system
  (if (> (`self.damage`) (`self.invertDamage`)) :!label _label
    (`self.AddMovementInput` _returnvalue_2 (* AxisValue -1.0))
    (`self.AddMovementInput` _returnvalue_3 (* (stale `InputAxis|strafeAxis` AxisValue) -1.0))
    (else
      (`self.AddMovementInput` _returnvalue_2 AxisValue)
      (`self.AddMovementInput` _returnvalue_3 (stale `InputAxis|strafeAxis` AxisValue)))))

(event `InputAxis|strafeAxis`
  (params (AxisValue :type "Float (single-precision)"))
  ;[1 1 1] Movement system
  (goto _label))

(event `self.ReceiveBeginPlay`
  (bind _returnvalue (`GameplayStatics.GetPlayerController` 0))
  ;[1 1 1] Set Camera and mouse
  (`PlayerController.SetViewTargetWithBlend` _returnvalue (`self.camera`) 0.0 "VTBlend_Linear" 0.0 false)
  (set `PlayerController.bShowMouseCursor` true _returnvalue)
  (set `self.damage` 0)
  (set `self.invertDamage` 5))

(event `self.ReceiveTick`
  (params (DeltaSeconds :type "Float (single-precision)"))
  (bind (_bblockinghit _binitialoverlap _time _distance _location) (`GameplayStatics.BreakHitResult` (`PlayerController.GetHitResultUnderCursorByChannel` (`GameplayStatics.GetPlayerController` 0) "TraceTypeQuery1" true)))
  (bind (_returnvalue_roll _returnvalue_pitch _returnvalue_yaw) (`KismetMathLibrary.BreakRotator` (`KismetMathLibrary.FindLookAtRotation` (`self.K2_GetActorLocation` (`GameplayStatics.GetPlayerController` 0)) _location)))
  ;[1 1 1] Rotate @ mouse
  (if _bblockinghit
    (`self.K2_SetActorRotation` self (`KismetMathLibrary.MakeRotator` 0.0 0.0 _returnvalue_yaw) false)
    (`SceneComponent.K2_SetWorldLocationAndRotation` :`self` (`Actor.RootComponent` (`self.decal`)) :`NewLocation` _location)))

(fn `UserConstructionScript`)